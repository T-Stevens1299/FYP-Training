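; BP_ParentUnit is a base pawn for a selectable, movable ship unit.
; Clicking it shows a Cylinder mesh and registers the unit with the first player controller through RegisterUnitMessage.
; A MovetoTarget event sends the pawn to a given location with AI MoveTo, while the construction script sets the FloatingPawnMovement max speed from ShipSpeed.
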(event `self.ReceiveActorOnClicked`
  (params (ButtonPressed :type "Key Structure"))
  (`SceneComponent.SetVisibility` (`self.Cylinder`) true false)
  (message `/Game/FYPContent/Interfaces/BPI_UnitSelection.RegisterUnit` (`GameplayStatics.GetPlayerController` 0) self))

(event `/Game/FYPContent/Interfaces/BPI_Targeting.MoveToTarget`
  (params (TargetLocation :type "Vector Structure"))
  (`|AIMoveTo` self TargetLocation null))

(fn `UserConstructionScript`
  (set `FloatingPawnMovement.MaxSpeed` (`self.ShipSpeed`) (`self.FloatingPawnMovement`)))