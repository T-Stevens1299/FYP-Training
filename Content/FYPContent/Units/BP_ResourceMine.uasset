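; BP_ResourceMine is a resource mine unit Blueprint that reports cursor hover to the first player controller.
; On init it binds cursor-over events, sending OnHoverMessage with its PlayerControlled value and itself on hover start, and ClearHoverMessage on hover end.
; Its unbind event targets BeginHover for both cursor events, so the EndHover binding is not removed.
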(event `self.unbindBlueprintEvents`
  (remove `Actor.OnBeginCursorOver` (delegate `BeginHover`))
  (remove `Actor.OnEndCursorOver` (delegate `BeginHover`)))

(event `self.initBlueprintScript`
  (add `Actor.OnBeginCursorOver` (delegate `BeginHover`))
  (add `Actor.OnEndCursorOver` (delegate `EndHover`)))

(event `BeginHover`
  (params (TouchedActor :type "Actor Object Reference"))
  (message `Interface_UnitSelection.OnHover` (`GameplayStatics.GetPlayerController` 0) (`self.playerControlled`) self))

(event `EndHover`
  (params (TouchedActor :type "Actor Object Reference"))
  (message `Interface_UnitSelection.ClearHover` (`GameplayStatics.GetPlayerController` 0)))

(fn `UserConstructionScript`)