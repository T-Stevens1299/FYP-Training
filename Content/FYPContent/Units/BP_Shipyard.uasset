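; BP_Shipyard is the shipyard unit, which reports cursor hover and selection to the player controller.
; On initialization it binds cursor-over events that send or clear a hover message, passing whether the shipyard is player-controlled.
; On click release it waits briefly, then, if player-controlled, registers itself with the controller as a unit and toggles its selection on.
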(event `self.initBlueprintScript`
  (add `Actor.OnBeginCursorOver` (delegate `BeginHover`))
  (add `Actor.OnEndCursorOver` (delegate `EndHover`)))

(event `BeginHover`
  (params (TouchedActor :type "Actor Object Reference"))
  (message `Interface_UnitSelection.OnHover` (`GameplayStatics.GetPlayerController` 0) (`self.playerControlled`) self))

(event `EndHover`
  (params (TouchedActor :type "Actor Object Reference"))
  (message `Interface_UnitSelection.ClearHover` (`GameplayStatics.GetPlayerController` 0)))

(event `self.ReceiveActorOnReleased`
  (params (ButtonReleased :type "Key Structure"))
  (`KismetSystemLibrary.Delay` 0.1)
  (if (`self.playerControlled`)
    (message `Interface_UnitSelection.RegisterUnit` (`GameplayStatics.GetPlayerController` 0) self)
    (`self.ToggleSelect` self true)))

(fn `UserConstructionScript`)