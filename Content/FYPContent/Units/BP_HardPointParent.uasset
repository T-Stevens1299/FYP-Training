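; Base hardpoint for a parent unit, acting as a targetable component with its own health and, optionally, a weapon.
; Damage updates health and notifies the parent, removing and destroying the hardpoint at zero.
; Weapons fire on a looping timer when a line trace passes range and self-hit arc checks, asking the parent to retarget once the target is gone.
; Cursor hover reports the hardpoint and its allegiance to the player controller.
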(event `self.ReceiveBeginPlay`
  (add `self.OnBeginCursorOver` (delegate `HoverBeing`))
  (add `self.OnEndCursorOver` (delegate `HoverEnd`)))

(event `HoverBeing` :!signature `self.OnBeginCursorOver`
  (params (TouchedActor :type "Actor Object Reference"))
  (message `/Game/FYPContent/Interfaces/BPI_UnitSelection.OnHover` (`GameplayStatics.GetPlayerController` 0) (`self.IsEnemy`) self))

(event `HoverEnd` :!signature `self.OnEndCursorOver`
  (params (TouchedActor :type "Actor Object Reference"))
  (message `/Game/FYPContent/Interfaces/BPI_UnitSelection.ClearHover` (`GameplayStatics.GetPlayerController` 0)))

(event `/Game/FYPContent/Interfaces/BPI_Damage.Damage`
  (params (DamageDealt :type "Float (double-precision)"))
  (bind _returnvalue (- (`self.CurrentHealth`) DamageDealt))
  (if (<= _returnvalue 0.0)
    (bind _asbp_parent_unit (cast `/Game/FYPContent/Units/BP_ParentUnit` (`self.HardpointParentUnit`)))
    (`KismetArrayLibrary.Array_RemoveItem` (`/Game/FYPContent/Units/BP_ParentUnit.Hardpoints` _asbp_parent_unit) self)
    (`KismetSystemLibrary.Delay` 0.2)
    (bind _hardpointparentunit (`self.HardpointParentUnit`)
      (:`then`
        (message `/Game/FYPContent/Interfaces/BPI_Damage.TriggerHealthCalculations` _hardpointparentunit)
        (`self.K2_DestroyActor`))
      (:`else`))
    (else
      (bind _output_get (set `self.CurrentHealth` _returnvalue))
      (`KismetSystemLibrary.PrintString` (`KismetStringLibrary.Concat_StrStr` "Hardpoint Health: " (`KismetStringLibrary.Conv_DoubleToString` _output_get)))
      (bind _hardpointparentunit_2 (`self.HardpointParentUnit`)
        (:`then`
          (message `/Game/FYPContent/Interfaces/BPI_Damage.TriggerHealthCalculations` _hardpointparentunit_2))
        (:`else`)))))

(event `/Game/FYPContent/Interfaces/BPI_Damage.SetHardpointTarget`
  (params (CurrentTarget :type "Actor Object Reference") (ActorsToIgnore :type "Array of Actor Object Reference (by ref)"))
  (if (`self.IsWeapon`)
    (set `self.CurrentTarget` CurrentTarget)
    (bind _returnvalue (`KismetSystemLibrary.K2_SetTimerDelegate` (delegate `FireWeapon`) (`self.FireRate`) true))
    (set `self.FireHandle` _returnvalue)))

(event `FireWeapon`
  (bind _canshoot (`self.CheckTargetRange` (stale `/Game/FYPContent/Interfaces/BPI_Damage.SetHardpointTarget` ActorsToIgnore)))
  (if _canshoot
    (bind _currenttarget (`self.CurrentTarget`)
      (:`then`
        (message `/Game/FYPContent/Interfaces/BPI_Damage.Damage` _currenttarget (`self.OutputDamage`)))
      (:`else`
        (`KismetSystemLibrary.K2_ClearAndInvalidateTimerHandle` (`self.FireHandle`))
        (message `/Game/FYPContent/Interfaces/BPI_Targeting.AttackExistingTarget` (`self.HardpointParentUnit`))))))

(fn `CheckTargetRange`
  (params (ActorsToIgnore :type "Array of Actor Object Reference"))
  (returns (CanShoot :type Boolean))
  (locals (Ignore :type "Array of Actor Object Reference"))
  (bind _output_get (set `local.Ignore` ActorsToIgnore))
  (`KismetArrayLibrary.Array_Remove` _output_get (`KismetArrayLibrary.Array_Find` _output_get self))
  (`self.CurrentTarget`
    (:`then`
      (`self.SetTargetsParent`)
      (bind _outhit (`KismetSystemLibrary.LineTraceSingle` (`SceneComponent.K2_GetComponentLocation` (`self.Fire Point`)) (`self.K2_GetActorLocation` (`self.CurrentTarget`)) "TraceTypeQuery1" false (`local.Ignore`) "ForDuration" false))
      (bind (_bblockinghit _binitialoverlap _time _distance _location _impactpoint _normal _impactnormal _physmat _hitactor) (`GameplayStatics.BreakHitResult` _outhit))
      ;[1 1 1] Checks to see if the it is in range to fire and in case it hit itself - invisible plane barrier dictates firing arc radius
      (if (== self _hitactor)
        _
        (elif (<= _distance (`self.WeaponRange`))
          (return true)
          (else
            (return false)))))
    (:`else`
      (`KismetSystemLibrary.K2_ClearAndInvalidateTimerHandle` (`self.FireHandle`)))))

(fn `Damage Calculations`
  (params (DamageTook :type "Float (double-precision)") (DamageCauser :type "Actor Object Reference"))
  (bind _returnvalue (- (`self.CurrentHealth`) DamageTook))
  (if (<= _returnvalue 0.0)
    (bind _asbp_parent_unit (cast `/Game/FYPContent/Units/BP_ParentUnit` (`self.HardpointParentUnit`)))
    (`KismetArrayLibrary.Array_RemoveItem` (`/Game/FYPContent/Units/BP_ParentUnit.Hardpoints` _asbp_parent_unit) self)
    (else
      (bind _output_get (set `self.CurrentHealth` _returnvalue))
      (bind _hardpointparentunit (`self.HardpointParentUnit`)
        (:`then`
          (message `/Game/FYPContent/Interfaces/BPI_Damage.TriggerHealthCalculations` _hardpointparentunit))
        (:`else`)))))

(fn `SetTargetsParent`
  ;[1 1 1] Sets the ship target for the auto targeting function
  (bind _asbp_hard_point_parent (cast `/Game/FYPContent/Units/BP_HardPointParent` (`self.CurrentTarget`)))
  (bind _asbp_parent_unit (cast `/Game/FYPContent/Units/BP_ParentUnit` (`self.HardpointParentUnit`)))
  (set `/Game/FYPContent/Units/BP_ParentUnit.CurrentShipTarget` (`/Game/FYPContent/Units/BP_HardPointParent.HardpointParentUnit` _asbp_hard_point_parent) _asbp_parent_unit))

(fn `UserConstructionScript`
  (set `self.CurrentHealth` (`self.TotalHealth`))
  (set `self.HardpointParentUnit` (`self.GetParentActor`)))