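; Destroyer unit pawn that can be hovered, selected and ordered to move or attack, with movement and turn speeds applied from its variables.
; On BeginPlay it gathers its bridge and gun child actors into a Hardpoints array and sets their parent.
; Cursor events message the player controller, and releasing a click on a player-controlled ship registers and selects it.
; Orders use AI MoveTo, with attack orders also setting the hardpoint target.
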(event `self.ReceiveBeginPlay`
  (add `self.OnBeginCursorOver` (delegate `BeginHover`))
  (add `self.OnEndCursorOver` (delegate `EndHover`))
  (`self.SetSpeeds`)
  (`self.GatherHardpoints`)
  (`self.setHardpointsParent`))

(event `BeginHover` :!signature `self.OnBeginCursorOver`
  (params (TouchedActor :type "Actor Object Reference"))
  (message `Interface_UnitSelection.OnHover` (`GameplayStatics.GetPlayerController` 0) (`self.playerControlled`) self))

(event `EndHover` :!signature `self.OnEndCursorOver`
  (params (TouchedActor :type "Actor Object Reference"))
  (message `Interface_UnitSelection.ClearHover` (`GameplayStatics.GetPlayerController` 0)))

(event `self.ReceiveActorOnReleased`
  (params (ButtonReleased :type "Key Structure"))
  (`KismetSystemLibrary.Delay` 0.1)
  (if (`self.playerControlled`)
    (message `Interface_UnitSelection.RegisterUnit` (`GameplayStatics.GetPlayerController` 0) self)
    (`self.ToggleSelect` self true)))

(event `self.moveObject`
  (params (Location :type "Vector Structure") (acceptanceRange :type "Float (single-precision)"))
  (`|AIMoveTo` self Location null acceptanceRange))

(event `self.moveToAttackTarget`
  (params (target :type "Actor Object Reference") (acceptanceRange :type "Float (single-precision)"))
  (`|AIMoveTo` self (0.0 0.0 0.0) target acceptanceRange
    (:`then`
      (`self.setHardpointTarget`))))

(fn `GatherHardpoints`
  (set `self.Hardpoints` (`|MakeArray` (`ChildActorComponent.ChildActor` (`self.HardpointBridge`)) (`ChildActorComponent.ChildActor` (`self.HardpointForwardGun1`)) (`ChildActorComponent.ChildActor` (`self.HardpointForwardGun2`)) (`ChildActorComponent.ChildActor` (`self.HardpointBackSideGun`)) (`ChildActorComponent.ChildActor` (`self.HardpointBackSideGun1`)) (`ChildActorComponent.ChildActor` (`self.HardpointBackSideGun2`)) (`ChildActorComponent.ChildActor` (`self.HardpointBackSideGun3`)))))

(fn `SetSpeeds`
  (bind _charactermovement (`self.CharacterMovement`))
  (set `CharacterMovementComponent.MaxWalkSpeed` (`self.UnitSpeed`) _charactermovement)
  (set `CharacterMovementComponent.RotationRate` (`KismetMathLibrary.MakeRotator` 0.0 0.0 (`self.UnitRotationSpeed`)) _charactermovement))

(fn `UserConstructionScript`)